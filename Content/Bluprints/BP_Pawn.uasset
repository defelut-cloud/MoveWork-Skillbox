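; BP_Pawn is an AI pawn that wanders endlessly around the navigable area of the level.
; On BeginPlay it caches the center and extent of the level's NavMeshBoundsVolume.
; It picks a random point in that box, projects it onto the navmesh with a tall vertical query extent and moves there with AIMoveTo.
; Both success and failure of the move trigger a new destination, forming a continuous loop.
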(event Custom|Move%20To%20Target
  (AI|AIMoveTo self (Variables|Default|GetTargetLocation) 0 5.0 false
    (:OnSuccess
      _)
    (:OnFail
      _))
  (CallFunction|GenerateNavCordinates))

(event Custom|GenerateNavCordinates
  (Variables|Default|SetTargetLocation (.ProjectedLocation (AI|Navigation|ProjectPointtoNavigation (Math|Random|RandomPointinBoundingBox (Variables|Default|GetNavMashCenter) (Variables|Default|GetNavMashBounds)) 0 0 "0.000000,0.000000,500.000000")))
  (CallFunction|MovetoTarget))

(event EventBeginPlay
  (bind _returnvalue (Actor|GetActorOfClass "/Script/NavigationSystem.NavMeshBoundsVolume"))
  (Variables|Default|SetNavMashCenter (.Origin (Collision|GetActorBounds _returnvalue false false)))
  (Variables|Default|SetNavMashBounds (.BoxExtent (Collision|GetActorBounds _returnvalue false false)))
  (CallFunction|GenerateNavCordinates))

(fn ConstructionScript)